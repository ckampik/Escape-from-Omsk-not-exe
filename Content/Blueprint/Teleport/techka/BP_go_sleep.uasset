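; BP_go_sleep is a trigger-box actor that shows a go-sleep prompt and sets up the next go-sleep point in the world.
; When BP_Character enters the box, it shows WBP_go_sleep and sets the character's IVisitMetro flag, removing the widget on exit.
; The first entry also spawns BP_marks and BP_go_sleep_HOUSE_new at hardcoded transforms, guarded by a Spawn boolean.
; The IVisitMetro check directly follows its assignment, so it always passes.
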(event OnComponentBeginOverlap(Box)
  (params (OverlappedComponent :type Primitive%20Component%20Object%20Reference) (OtherActor :type Actor%20Object%20Reference) (OtherComp :type Primitive%20Component%20Object%20Reference) (OtherBodyIndex :type Integer) (bFromSweep :type Boolean) (SweepResult :type Hit%20Result%20Structure%20%28by%20ref%29))
  (bind _asbp_character (Utilities|Casting|CastToBP_Character OtherActor))
  (bind _returnvalue (UserInterface|CreateWidget "/Game/Blueprint/Teleport/techka/WBP_go_sleep.WBP_go_sleep_C"))
  (UserInterface|Viewport|AddtoViewport _returnvalue 0)
  (Variables|/Game/Blueprint/Main_Character/BP_Character.BP_Character_C|SetiVisitMetro? _asbp_character true)
  (if (Variables|/Game/Blueprint/Main_Character/BP_Character.BP_Character_C|GetiVisitMetro? _asbp_character)
    (if (not (Variables|Default|Getspawn))
      (Game|SpawnActorfromClass "/Game/Blueprint/Markers/BP_marks.BP_marks_C" (Math|Transform|MakeTransform "4770.000000,0.000000,-910.000000" "0, 0, 0" "1.000000,1.000000,1.000000") "Undefined" "MultiplyWithRoot" 0 0)
      (Game|SpawnActorfromClass "/Game/Blueprint/Teleport/sleep/BP_go_sleep_HOUSE_new.BP_go_sleep_HOUSE_new_C" (Math|Transform|MakeTransform "4760.000000,0.000000,-1010.000000" "0, 0, 0" "2.250000,3.500000,2.500000") "Undefined" "MultiplyWithRoot" 0 0)
      (Variables|Default|Setspawn true))))

(event OnComponentEndOverlap(Box)
  (params (OverlappedComponent :type Primitive%20Component%20Object%20Reference) (OtherActor :type Actor%20Object%20Reference) (OtherComp :type Primitive%20Component%20Object%20Reference) (OtherBodyIndex :type Integer))
  (Utilities|Casting|CastToBP_Character OtherActor)
  (Widget|RemovefromParent (stale OnComponentBeginOverlap(Box) _returnvalue)))

(event EventBeginPlay)

(event Collision|EventActorBeginOverlap
  (params (OtherActor :type Actor%20Object%20Reference)))

(event EventTick
  (params (DeltaSeconds :type Float%20%28single-precision%29)))

(fn ConstructionScript)