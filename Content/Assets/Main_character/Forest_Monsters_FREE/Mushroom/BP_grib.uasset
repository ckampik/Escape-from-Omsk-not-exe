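; Mushroom enemy for a 2D side-scroller that patrols, hurts the player on contact and can be killed.
; Tick drives a step-counter patrol, flipping the sprite and direction at each limit unless movement is locked.
; Box overlap plays an attack, damages the player, records its X for them and recoils away.
; Taking damage triggers knockback and a brief stun, or death, which destroys it and increments BP_Character's kill count.
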(event OnComponentBeginOverlap(Box)
  (params (OverlappedComponent :type Primitive%20Component%20Object%20Reference) (OtherActor :type Actor%20Object%20Reference) (OtherComp :type Primitive%20Component%20Object%20Reference) (OtherBodyIndex :type Integer) (bFromSweep :type Boolean) (SweepResult :type Hit%20Result%20Structure%20%28by%20ref%29))
  ;[0 0.002576 1] Damage
  (if (== OtherActor (Variables|Default|GetAs%20BP%20Character))
    (if (not (Variables|Default|GetisDead))
      (Variables|Default|SetisMovementLock true)
      (Class|PaperZDAnimInstance|JumptoNode (Variables|/Script/PaperZD.PaperZDAnimationComponent|GetAnimInstance (Variables|Default|GetAnimationComponent)) "rip" "None")
      (Utilities|FlowControl|Delay 0.25)
      (Variables|/Game/Blueprint/Main_Character/BP_Character.BP_Character_C|SetEnemyPosition (Variables|Default|GetAs%20BP%20Character) (.x (Transformation|GetWorldLocation (Variables|Default|GetSprite))))
      (Game|Damage|ApplyDamage OtherActor 1e+01 0 0)
      (Development|PrintString "получил")
      (Math|Float|CompareFloat (.x (Transformation|GetWorldLocation (Variables|/Script/Paper2D.PaperCharacter|GetSprite (Variables|Default|GetAs%20BP%20Character)))) (.x (Transformation|GetWorldLocation (Variables|Default|GetSprite)))
        (:>
          (Character|LaunchCharacter "-500.000000,0.000000,0.000000" true false))
        (:<
          (Character|LaunchCharacter "500.000000,0.000000,0.000000" true false)))
      (Variables|/Game/Blueprint/Main_Character/BP_Character.BP_Character_C|SetEnemyPosition (Variables|Default|GetAs%20BP%20Character) (.x (Transformation|GetWorldLocation (Variables|Default|GetSprite))))
      (Variables|Default|SetisMovementLock true)
      (Utilities|FlowControl|Delay 0.75)
      (Variables|Default|SetisMovementLock false))))

(event Custom|walkOnLock
  ;[0 0 0] walk
  (if (not (Variables|Default|GetisMovementLock))
    (Math|Float|CompareFloat (Variables|Default|Gets1) (Variables|Default|Gets)
      (:>
        (Pawn|Input|AddMovementInput "-1.000000,0.000000,0.000000" 1.0 false)
        (Variables|Default|Sets1 (- (Variables|Default|Gets1) 1.0)))
      (:==
        (if (> (Variables|Default|Gets) 0.0)
          (Variables|Default|Sets (* (Variables|Default|Gets) -1.0))
          (Variables|Default|Sets1 0.0)
          (Transformation|SetRelativeRotation (Variables|Default|GetSprite) "0, 0, 0" false false)
          (else
            (Variables|Default|Sets (* (Variables|Default|Gets) -1.0))
            (Variables|Default|Sets1 0.0)
            (Transformation|SetRelativeRotation (Variables|Default|GetSprite) "0.000000,180.000000,0.000000" false false))))
      (:<
        (Pawn|Input|AddMovementInput "1.000000,0.000000,0.000000" 1.0 false)
        (Variables|Default|Sets1 (+ (Variables|Default|Gets1) 1.0))))))

(event EventBeginPlay
  (bind _asbp_character (Utilities|Casting|CastToBP_Character (Game|GetPlayerCharacter 0)))
  (Variables|Default|SetAs%20BP%20Character _asbp_character))

(event Collision|EventActorBeginOverlap
  (params (OtherActor :type Actor%20Object%20Reference)))

(event EventTick
  (params (DeltaSeconds :type Float%20%28single-precision%29))
  (CallFunction|WalkonLock))

(event Game|Damage|EventAnyDamage
  (params (Damage :type Float%20%28single-precision%29) (DamageType :type Damage%20Type%20Object%20Reference) (InstigatedBy :type Controller%20Object%20Reference) (DamageCauser :type Actor%20Object%20Reference))
  (if (not (Variables|Default|GetisDead))
    (Class|PaperZDAnimInstance|JumptoNode (Variables|/Script/PaperZD.PaperZDAnimationComponent|GetAnimInstance (Variables|Default|GetAnimationComponent)) "hit" "None")
    (Math|Float|CompareFloat (.x (Transformation|GetWorldLocation (Variables|/Script/Paper2D.PaperCharacter|GetSprite (Variables|Default|GetAs%20BP%20Character)))) (.x (Transformation|GetWorldLocation (Variables|Default|GetSprite)))
      (:>
        (Character|LaunchCharacter "-500.000000,0.000000,100.000000" true true))
      (:<
        (Character|LaunchCharacter "500.000000,0.000000,100.000000" true true)))
    (Variables|Default|Sethealth (- (Variables|Default|Gethealth) Damage))
    (if (< (Variables|Default|Gethealth) 0.0)
      (Variables|Default|SetisMovementLock true)
      (Variables|Default|SetisDead true)
      (Class|PaperZDAnimInstance|JumptoNode (Variables|/Script/PaperZD.PaperZDAnimationComponent|GetAnimInstance (Variables|Default|GetAnimationComponent)) "Dead" "None")
      (Utilities|FlowControl|Delay 1.5)
      (Actor|DestroyActor)
      (bind _asbp_character (Utilities|Casting|CastToBP_Character (Game|GetPlayerCharacter 0)))
      (Variables|/Game/Blueprint/Main_Character/BP_Character.BP_Character_C|SethowIkillgrib _asbp_character (+ (Variables|/Game/Blueprint/Main_Character/BP_Character.BP_Character_C|GethowIkillgrib _asbp_character) 1))
      (else
        (Variables|Default|SetisMovementLock true)
        (Utilities|FlowControl|Delay 1.0)
        (Variables|Default|SetisMovementLock false)))))

(fn ConstructionScript)