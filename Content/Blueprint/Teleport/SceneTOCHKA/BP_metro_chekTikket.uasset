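; Metro ticket-check trigger that starts TOCHKA scene 1 while the SaveScene1 save exists with Scene1 unset.
; On BeginPlay it spawns a BP_marks marker at its box, whose overlap plays a sound, shows a ticket dialog and enables input.
; Pressing E once opens the scene widget and locks character input.
; A 0.2-second Delay loop polls the character's Scene1 flag, then restores input and writes a new save.
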(event OnComponentBeginOverlap(Box)
  (params (OverlappedComponent :type Primitive%20Component%20Object%20Reference) (OtherActor :type Actor%20Object%20Reference) (OtherComp :type Primitive%20Component%20Object%20Reference) (OtherBodyIndex :type Integer) (bFromSweep :type Boolean) (SweepResult :type Hit%20Result%20Structure%20%28by%20ref%29))
  (Utilities|Casting|CastToBP_Character OtherActor)
  (bind _returnvalue (SaveGame|DoesSaveGameExist "SaveScene1"))
  (if _returnvalue
    (bind _returnvalue_2 (SaveGame|LoadGamefromSlot "SaveScene1"))
    (bind _asbp_save_main_character (Utilities|Casting|CastToBP_saveMainCharacter _returnvalue_2))
    (if (not (Variables|/Game/Blueprint/Main_Character/BP_saveMainCharacter.BP_saveMainCharacter_C|Getscene1 _asbp_save_main_character))
      (Audio|PlaySound2D "/Game/Blueprint/Teleport/widget_subtitri/Speakers/Gta5_sound.Gta5_sound" 1.0 1.0 0.0 0 0)
      (bind _returnvalue_3 (UserInterface|CreateWidget "/Game/Blueprint/Teleport/WereTicket/WBP_dialogWereTicket.WBP_dialogWereTicket_C"))
      (UserInterface|Viewport|AddtoViewport _returnvalue_3 0)
      (Input|EnableInput (Game|GetPlayerController 0)))))

(event OnComponentEndOverlap(Box)
  (params (OverlappedComponent :type Primitive%20Component%20Object%20Reference) (OtherActor :type Actor%20Object%20Reference) (OtherComp :type Primitive%20Component%20Object%20Reference) (OtherBodyIndex :type Integer))
  (Utilities|Casting|CastToBP_Character OtherActor)
  (Widget|RemovefromParent (stale OnComponentBeginOverlap(Box) _returnvalue_3))
  (Input|DisableInput (Game|GetPlayerController 0)))

(event EventBeginPlay
  (Utilities|Casting|CastToBP_Character (Game|GetPlayerCharacter 0))
  (bind _returnvalue (SaveGame|DoesSaveGameExist "SaveScene1"))
  (if _returnvalue
    (bind _returnvalue_2 (SaveGame|LoadGamefromSlot "SaveScene1"))
    (bind _asbp_save_main_character (Utilities|Casting|CastToBP_saveMainCharacter _returnvalue_2))
    (if (not (Variables|/Game/Blueprint/Main_Character/BP_saveMainCharacter.BP_saveMainCharacter_C|Getscene1 _asbp_save_main_character))
      (Game|SpawnActorfromClass "/Game/Blueprint/Markers/BP_marks.BP_marks_C" (Math|Conversions|ToTransform(Vector) (Transformation|GetWorldLocation (Variables|Default|GetBox))) "Undefined" "MultiplyWithRoot" 0 0))))

(event Input|KeyboardEvents|E
  (params (Key :type Key%20Structure :default "None"))
  (:Pressed
    (if (not (Variables|Default|Getb))
      (Variables|Default|Setb true)
      (Widget|RemovefromParent (stale OnComponentBeginOverlap(Box) _returnvalue_3))
      (bind _asbp_character (Utilities|Casting|CastToBP_Character (Game|GetPlayerCharacter 0)))
      (Input|DisableInput _asbp_character (Game|GetPlayerController 0))
      (bind _returnvalue (UserInterface|CreateWidget "/Game/Blueprint/Teleport/SceneTOCHKA/WBP_TOCHKA_scene_1.WBP_TOCHKA_scene_1_C"))
      (UserInterface|Viewport|AddtoViewport _returnvalue 0)
      (if (Variables|/Game/Blueprint/Main_Character/BP_Character.BP_Character_C|Getscene1 _asbp_character) :!label _label
        (Input|EnableInput _asbp_character 0)
        (bind _returnvalue_2 (SaveGame|CreateSaveGameObject "/Game/Blueprint/Main_Character/BP_saveMainCharacter.BP_saveMainCharacter_C"))
        (Variables|/Game/Blueprint/Main_Character/BP_saveMainCharacter.BP_saveMainCharacter_C|Setscene1 _returnvalue_2 (Variables|/Game/Blueprint/Main_Character/BP_Character.BP_Character_C|Getscene1 _asbp_character))
        (SaveGame|SaveGametoSlot _returnvalue_2 "SaveScene1")
        (else
          (Utilities|FlowControl|Delay 0.2)
          (goto _label))))))

(fn ConstructionScript)