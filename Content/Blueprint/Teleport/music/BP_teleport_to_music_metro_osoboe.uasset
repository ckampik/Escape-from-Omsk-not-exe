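; Trigger-box teleporter that sends the player to the Metro_Music level, gated by the Gitardialog flag in the "gitarDialog" save slot.
; When BP_Character enters and the flag is set, it shows a prompt widget and enables input on itself.
; Pressing E adds a fade widget, then opens the level after a short delay.
; Leaving the box removes the prompt and disables input.
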(event OnComponentBeginOverlap(Box)
  (params (OverlappedComponent :type Primitive%20Component%20Object%20Reference) (OtherActor :type Actor%20Object%20Reference) (OtherComp :type Primitive%20Component%20Object%20Reference) (OtherBodyIndex :type Integer) (bFromSweep :type Boolean) (SweepResult :type Hit%20Result%20Structure%20%28by%20ref%29))
  (Utilities|Casting|CastToBP_Character OtherActor)
  (bind _returnvalue (SaveGame|DoesSaveGameExist "gitarDialog"))
  (if _returnvalue
    (bind _returnvalue_2 (SaveGame|LoadGamefromSlot "gitarDialog"))
    (bind _asbp_save_main_character (Utilities|Casting|CastToBP_saveMainCharacter _returnvalue_2))
    (if (Variables|/Game/Blueprint/Main_Character/BP_saveMainCharacter.BP_saveMainCharacter_C|Getgitardialog _asbp_save_main_character)
      (bind _returnvalue_3 (UserInterface|CreateWidget "/Game/Blueprint/Teleport/music/WBP_music_to_metro.WBP_music_to_metro_C"))
      (UserInterface|Viewport|AddtoViewport _returnvalue_3 0)
      (Input|EnableInput (Game|GetPlayerController 0)))))

(event OnComponentEndOverlap(Box)
  (params (OverlappedComponent :type Primitive%20Component%20Object%20Reference) (OtherActor :type Actor%20Object%20Reference) (OtherComp :type Primitive%20Component%20Object%20Reference) (OtherBodyIndex :type Integer))
  (Utilities|Casting|CastToBP_Character OtherActor)
  (Widget|RemovefromParent (stale OnComponentBeginOverlap(Box) _returnvalue_3))
  (Input|DisableInput (Game|GetPlayerController 0)))

(event EventBeginPlay)

(event Collision|EventActorBeginOverlap
  (params (OtherActor :type Actor%20Object%20Reference)))

(event EventTick
  (params (DeltaSeconds :type Float%20%28single-precision%29)))

(event Input|KeyboardEvents|E
  (params (Key :type Key%20Structure :default "None"))
  (:Pressed
    (bind _returnvalue (UserInterface|CreateWidget "/Game/Blueprint/Teleport/WBP_fade.WBP_fade_C"))
    (UserInterface|Viewport|AddtoViewport _returnvalue 0)
    (Utilities|FlowControl|Sequence
      (:then_0
        (Utilities|FlowControl|Delay 1.8)
        (Game|OpenLevel(byName) "Metro_Music"))
      (:then_1
        (Utilities|FlowControl|Delay 2.0)
        (Widget|RemovefromParent (stale OnComponentBeginOverlap(Box) _returnvalue_3))))))

(fn ConstructionScript)