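; BP_trampline is a trampoline that launches BP_Character straight up when it overlaps the Cube component.
; On overlap it requests a jump to the JumpAction anim node, plays a 2D sound and calls LaunchCharacter, overriding existing velocity.
; The custom Jump event runs a timeline that moves the Cube along local Z between rest and a lowered position.
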(event OnComponentBeginOverlap(Cube)
  (params (OverlappedComponent :type Primitive%20Component%20Object%20Reference) (OtherActor :type Actor%20Object%20Reference) (OtherComp :type Primitive%20Component%20Object%20Reference) (OtherBodyIndex :type Integer) (bFromSweep :type Boolean) (SweepResult :type Hit%20Result%20Structure%20%28by%20ref%29))
  (bind _asbp_character (Utilities|Casting|CastToBP_Character OtherActor))
  (Class|PaperZDAnimInstance|JumptoNode (Variables|/Script/PaperZD.PaperZDAnimationComponent|GetAnimInstance (Variables|/Script/PaperZD.PaperZDCharacter|GetAnimationComponent _asbp_character)) "JumpAction" "None")
  (CallFunction|Jump)
  (Audio|PlaySound2D "/Game/MusicSound/jumpgrib.jumpgrib" 1.0 1.0 0.0 0 0)
  (Character|LaunchCharacter _asbp_character "0.000000,0.000000,1500.000000" true true))

(event Custom|Jump
  (bind _alpha (Timeline|Timeline_jump PlayFromStart)
    (:Update
      (Transformation|SetRelativeLocation (Variables|Default|GetCube) (Math|Vector|MakeVector 0.0 0.0 (Math|Float|Lerp 0.0 -1e+02 _alpha)) false false))))

(fn ConstructionScript)