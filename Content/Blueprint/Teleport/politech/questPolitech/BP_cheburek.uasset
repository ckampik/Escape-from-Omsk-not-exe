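; Edible cheburek for the Politech quest that triggers a slow-motion mushroom hallucination when the player eats it.
; Box overlap shows prompt widgets and enables input; pressing E plays a sound, adds post-process effects and halves global time dilation.
; A delayed loop spawns BP_grib pairs in two diverging rows up to GribMax.
; It then polls BP_Character's kill count until GribMaxKill, restoring time and removing the effects.
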(event OnComponentBeginOverlap(Box)
  (params (OverlappedComponent :type Primitive%20Component%20Object%20Reference) (OtherActor :type Actor%20Object%20Reference) (OtherComp :type Primitive%20Component%20Object%20Reference) (OtherBodyIndex :type Integer) (bFromSweep :type Boolean) (SweepResult :type Hit%20Result%20Structure%20%28by%20ref%29))
  (if (not (Variables|Default|GetEat))
    (Utilities|Casting|CastToBP_Character OtherActor)
    (bind _returnvalue (UserInterface|CreateWidget "/Game/Blueprint/Teleport/politech/questPolitech/WBP_BP_cheburek.WBP_BP_cheburek_C"))
    (UserInterface|Viewport|AddtoViewport _returnvalue 0)
    (bind _returnvalue_2 (UserInterface|CreateWidget "/Game/Blueprint/Teleport/politech/questPolitech/WBP_cheburek.WBP_cheburek_C"))
    (UserInterface|Viewport|AddtoViewport _returnvalue_2 0)
    (Input|EnableInput (Game|GetPlayerController 0))))

(event OnComponentEndOverlap(Box)
  (params (OverlappedComponent :type Primitive%20Component%20Object%20Reference) (OtherActor :type Actor%20Object%20Reference) (OtherComp :type Primitive%20Component%20Object%20Reference) (OtherBodyIndex :type Integer))
  (Utilities|Casting|CastToBP_Character OtherActor)
  (Widget|RemovefromParent (stale OnComponentBeginOverlap(Box) _returnvalue))
  (Input|DisableInput (Game|GetPlayerController 0)))

(event Input|KeyboardEvents|E
  (params (Key :type Key%20Structure :default "None"))
  (:Pressed
    (if (not (Variables|Default|GetEat))
      (Widget|RemovefromParent (stale OnComponentBeginOverlap(Box) _returnvalue))
      (Variables|Default|SetEat true)
      (Audio|PlaySound2D "/Game/Blueprint/Teleport/politech/questPolitech/bolitJivot.bolitJivot" 1.0 1.0 0.0 0 0)
      (Utilities|FlowControl|Delay 1.0)
      (bind _returnvalue (UserInterface|CreateWidget "/Game/Blueprint/Teleport/politech/questPolitech/WBP_postProcces.WBP_postProcces_C"))
      (UserInterface|Viewport|AddtoViewport _returnvalue 0)
      (Utilities|FlowControl|Delay 1.0)
      (bind _returnvalue_2 (Game|SpawnActorfromClass "/Game/Blueprint/Teleport/politech/questPolitech/BP_post.BP_post_C" (Math|Conversions|ToTransform(Vector) (Transformation|GetWorldLocation (Variables|Default|GetBox))) "Undefined" "MultiplyWithRoot" 0 0))
      (Utilities|Time|SetGlobalTimeDilation 0.5)
      (Utilities|FlowControl|Delay 1.0)
      (if (Variables|Default|GetEat)
        (if (< (Variables|Default|GetGrib) (Variables|Default|GetGrib_max)) :!label _label
          (Game|SpawnActorfromClass "/Game/Assets/Main_character/Forest_Monsters_FREE/Mushroom/BP_grib.BP_grib_C" (Math|Transform|MakeTransform (Math|Vector|MakeVector (Variables|Default|GetgribSpawnX) (Variables|Default|GetgribSpawnY) -3.7e+02) "0, 0, 0" "1.000000,1.000000,1.000000") "AlwaysSpawn" "MultiplyWithRoot" 0 0)
          (Game|SpawnActorfromClass "/Game/Assets/Main_character/Forest_Monsters_FREE/Mushroom/BP_grib.BP_grib_C" (Math|Transform|MakeTransform (Math|Vector|MakeVector (Variables|Default|GetgribSpawnXLeft) (Variables|Default|GetgribSpawnYLeft) -3.7e+02) "0, 0, 0" "1.000000,1.000000,1.000000") "AlwaysSpawn" "MultiplyWithRoot" 0 0)
          (Variables|Default|SetgribSpawnX (+ (Variables|Default|GetgribSpawnX) 1.2e+02))
          (Variables|Default|SetgribSpawnY (+ (Variables|Default|GetgribSpawnY) 4e+01))
          (Variables|Default|SetgribSpawnXLeft (+ (Variables|Default|GetgribSpawnXLeft) -1.2e+02))
          (Variables|Default|SetgribSpawnYLeft (+ (Variables|Default|GetgribSpawnYLeft) 4e+01))
          (bind _result (Math|Integer|IncrementInt (stale _output_get))
            (:%20%20
              (bind _output_get (Variables|Default|SetGrib _result))
              (Utilities|FlowControl|Delay 0.5)
              (goto _label)))
          (else
            (bind _asbp_character (Utilities|Casting|CastToBP_Character (Game|GetPlayerCharacter 0) :!label _label_2))
            (if (!= (Variables|/Game/Blueprint/Main_Character/BP_Character.BP_Character_C|GethowIkillgrib _asbp_character) (Variables|Default|GetGrib_max_kill))
              (Utilities|FlowControl|Delay 0.2)
              (goto _label_2)
              (else
                (Utilities|Time|SetGlobalTimeDilation 1.0)
                (Variables|Default|SetEat false)
                (Variables|/Game/Blueprint/Main_Character/BP_Character.BP_Character_C|SethowIkillgrib _asbp_character 0)
                (Widget|RemovefromParent _returnvalue)
                (Actor|DestroyActor _returnvalue_2)))))))))

(fn ConstructionScript)