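; BP_politechStudents is a trigger actor for the one-time politech students scene, gated by the SceneStudents flag in the SaveScene3 save slot.
; On BeginPlay, an existing save with the flag unset spawns a BP_marks marker at the box.
; Player overlap under that condition disables input and shows WBP_politechStudents1.
; A 0.2-second Delay loop polls the character's flag, then restores input, destroys the trigger and saves the flag into a new save object.
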(event OnComponentBeginOverlap(Box)
  (params (OverlappedComponent :type Primitive%20Component%20Object%20Reference) (OtherActor :type Actor%20Object%20Reference) (OtherComp :type Primitive%20Component%20Object%20Reference) (OtherBodyIndex :type Integer) (bFromSweep :type Boolean) (SweepResult :type Hit%20Result%20Structure%20%28by%20ref%29))
  (Utilities|Casting|CastToBP_Character OtherActor)
  ;[0 0 0] BRANCH SAVE
  (bind _returnvalue (SaveGame|DoesSaveGameExist "SaveScene3"))
  (if _returnvalue
    (bind _returnvalue_2 (SaveGame|LoadGamefromSlot "SaveScene3"))
    (bind _asbp_save_main_character (Utilities|Casting|CastToBP_saveMainCharacter _returnvalue_2))
    (if (not (Variables|/Game/Blueprint/Main_Character/BP_saveMainCharacter.BP_saveMainCharacter_C|GetsceneStudents _asbp_save_main_character))
      (bind _asbp_character (Utilities|Casting|CastToBP_Character (Game|GetPlayerCharacter 0)))
      (Input|DisableInput _asbp_character (Game|GetPlayerController 0))
      (bind _returnvalue_3 (UserInterface|CreateWidget "/Game/Blueprint/Teleport/politechStudents/WBP_politechStudents1.WBP_politechStudents1_C"))
      (UserInterface|Viewport|AddtoViewport _returnvalue_3 0)
      (if (Variables|/Game/Blueprint/Main_Character/BP_Character.BP_Character_C|GetsceneStudents _asbp_character) :!label _label
        (Input|EnableInput _asbp_character 0)
        (Actor|DestroyActor)
        (bind _returnvalue_4 (SaveGame|CreateSaveGameObject "/Game/Blueprint/Main_Character/BP_saveMainCharacter.BP_saveMainCharacter_C"))
        (Variables|/Game/Blueprint/Main_Character/BP_saveMainCharacter.BP_saveMainCharacter_C|SetsceneStudents _returnvalue_4 (Variables|/Game/Blueprint/Main_Character/BP_Character.BP_Character_C|GetsceneStudents _asbp_character))
        (SaveGame|SaveGametoSlot _returnvalue_4 "SaveScene3")
        (else
          (Utilities|FlowControl|Delay 0.2)
          (goto _label))))))

(event EventBeginPlay
  (Utilities|Casting|CastToBP_Character (Game|GetPlayerCharacter 0))
  ;[0 0 0] BRANCH SAVE
  (bind _returnvalue (SaveGame|DoesSaveGameExist "SaveScene3"))
  (if _returnvalue
    (bind _returnvalue_2 (SaveGame|LoadGamefromSlot "SaveScene3"))
    (bind _asbp_save_main_character (Utilities|Casting|CastToBP_saveMainCharacter _returnvalue_2))
    (if (not (Variables|/Game/Blueprint/Main_Character/BP_saveMainCharacter.BP_saveMainCharacter_C|GetsceneStudents _asbp_save_main_character))
      (Game|SpawnActorfromClass "/Game/Blueprint/Markers/BP_marks.BP_marks_C" (Math|Conversions|ToTransform(Vector) (Transformation|GetWorldLocation (Variables|Default|GetBox))) "Undefined" "MultiplyWithRoot" 0 0))))

(fn ConstructionScript)