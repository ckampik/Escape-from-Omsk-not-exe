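; Slow-motion trigger for the flying-note moment, active while the "poimka" save's NePaimal flag is false.
; On BeginPlay it spawns a BP_list at a fixed spot.
; When BP_Character enters the Box, it sets global time dilation to 0.2 without restoring it, swaps the list for a short-lived BP_noteFly and plays a paper sound.
; A separate Jump event lowers the Box through a timeline.
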(event OnComponentBeginOverlap(Box)
  (params (OverlappedComponent :type Primitive%20Component%20Object%20Reference) (OtherActor :type Actor%20Object%20Reference) (OtherComp :type Primitive%20Component%20Object%20Reference) (OtherBodyIndex :type Integer) (bFromSweep :type Boolean) (SweepResult :type Hit%20Result%20Structure%20%28by%20ref%29))
  (Utilities|Casting|CastToBP_Character OtherActor)
  (bind _returnvalue (SaveGame|LoadGamefromSlot "poimka"))
  (bind _asbp_save_main_character (Utilities|Casting|CastToBP_saveMainCharacter _returnvalue))
  (if (not (Variables|/Game/Blueprint/Main_Character/BP_saveMainCharacter.BP_saveMainCharacter_C|GetnePaimal _asbp_save_main_character))
    (Utilities|Time|SetGlobalTimeDilation 0.2)
    (bind _returnvalue_2 (Game|SpawnActorfromClass "/Game/Blueprint/TakeNotes/BP_noteFly.BP_noteFly_C" (Math|Transform|MakeTransform "-730.000000,80.000000,-20.000000" "0, 0, 0" "0.188237,-0.561763,0.188237") "Undefined" "MultiplyWithRoot" 0 0))
    (Actor|DestroyActor (stale EventBeginPlay _returnvalue_3))
    (Utilities|FlowControl|Delay 0.25)
    (Audio|PlaySound2D "/Game/MusicSound/bumaga.bumaga" 1.0 1.0 0.0 0 0)
    (Utilities|FlowControl|Delay 2.0)
    (Actor|DestroyActor _returnvalue_2)))

(event Custom|Jump
  (bind _alpha (Timeline|Timeline PlayFromStart)
    (:Update
      (Transformation|SetRelativeLocation (Variables|Default|GetBox) (Math|Vector|MakeVector 0.0 0.0 (Math|Float|Lerp 0.0 -1e+02 _alpha)) false false))))

(event EventBeginPlay
  (bind _returnvalue (SaveGame|DoesSaveGameExist "poimka"))
  (if _returnvalue
    (bind _returnvalue_2 (SaveGame|LoadGamefromSlot "poimka"))
    (bind _asbp_save_main_character (Utilities|Casting|CastToBP_saveMainCharacter _returnvalue_2))
    (if (not (Variables|/Game/Blueprint/Main_Character/BP_saveMainCharacter.BP_saveMainCharacter_C|GetnePaimal _asbp_save_main_character))
      (bind _returnvalue_3 (Game|SpawnActorfromClass "/Game/Blueprint/TakeNotes/BP_list.BP_list_C" (Math|Transform|MakeTransform "-730.000000,-20.000000,-20.000000" "0, 0, 0" "0.188237,-0.561763,0.188237") "Undefined" "MultiplyWithRoot" 0 0)))))

(fn ConstructionScript)