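; BP_sleepOrNO is a sleep interaction trigger for the player character.
; Entering its Box shows one of two prompt widgets depending on the character's ISleep flag, and enables input only when not yet slept.
; Pressing E then plays a fade widget, sets ISleep after a delay, spawns BP_go_sleep_OUT_new at a fixed location and removes the widgets.
; Leaving the Box clears the prompts and disables input.
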(event OnComponentBeginOverlap(Box)
  (params (OverlappedComponent :type Primitive%20Component%20Object%20Reference) (OtherActor :type Actor%20Object%20Reference) (OtherComp :type Primitive%20Component%20Object%20Reference) (OtherBodyIndex :type Integer) (bFromSweep :type Boolean) (SweepResult :type Hit%20Result%20Structure%20%28by%20ref%29))
  (bind _asbp_character (Utilities|Casting|CastToBP_Character OtherActor))
  (if (Variables|/Game/Blueprint/Main_Character/BP_Character.BP_Character_C|GetiSleep _asbp_character)
    (bind _returnvalue (UserInterface|CreateWidget "/Game/Blueprint/Teleport/sleep/WBP_iSleep.WBP_iSleep_C"))
    (UserInterface|Viewport|AddtoViewport _returnvalue 0)
    (else
      (bind _returnvalue_2 (UserInterface|CreateWidget "/Game/Blueprint/Teleport/sleep/WBP_iSleep1.WBP_iSleep1_C"))
      (UserInterface|Viewport|AddtoViewport _returnvalue_2 0)
      (Input|EnableInput (Game|GetPlayerController 0)))))

(event OnComponentEndOverlap(Box)
  (params (OverlappedComponent :type Primitive%20Component%20Object%20Reference) (OtherActor :type Actor%20Object%20Reference) (OtherComp :type Primitive%20Component%20Object%20Reference) (OtherBodyIndex :type Integer))
  (Utilities|Casting|CastToBP_Character OtherActor)
  (Widget|RemovefromParent (stale OnComponentBeginOverlap(Box) _returnvalue_2))
  (Widget|RemovefromParent (stale OnComponentBeginOverlap(Box) _returnvalue))
  (Input|DisableInput (Game|GetPlayerController 0)))

(event EventBeginPlay)

(event Collision|EventActorBeginOverlap
  (params (OtherActor :type Actor%20Object%20Reference)))

(event EventTick
  (params (DeltaSeconds :type Float%20%28single-precision%29)))

(event Input|KeyboardEvents|E
  (params (Key :type Key%20Structure :default "None"))
  (:Pressed
    (if (not (Variables|/Game/Blueprint/Main_Character/BP_Character.BP_Character_C|GetiSleep (stale OnComponentBeginOverlap(Box) _asbp_character)))
      (bind _returnvalue (UserInterface|CreateWidget "/Game/Blueprint/Teleport/WBP_fade.WBP_fade_C"))
      (UserInterface|Viewport|AddtoViewport _returnvalue 0)
      (Utilities|FlowControl|Sequence
        (:then_0
          (Utilities|FlowControl|Delay 1.8)
          (bind _asbp_character (Utilities|Casting|CastToBP_Character (Game|GetPlayerCharacter 0)))
          (Variables|/Game/Blueprint/Main_Character/BP_Character.BP_Character_C|SetiSleep _asbp_character true)
          (Game|SpawnActorfromClass "/Game/Blueprint/Teleport/sleep/BP_go_sleep_OUT_new.BP_go_sleep_OUT_new_C" (Math|Transform|MakeTransform "2860.000000,0.000000,-2130.000000" "0, 0, 0" "1.750000,4.000000,1.750000") "Undefined" "MultiplyWithRoot" 0 0))
        (:then_1
          (Utilities|FlowControl|Delay 2.0)
          (Widget|RemovefromParent (stale OnComponentBeginOverlap(Box) _returnvalue_2)))))))

(fn ConstructionScript)