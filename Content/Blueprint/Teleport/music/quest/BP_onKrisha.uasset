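; Roof trigger for a music quest that stages dialogue from saved progress and spawns a BP_marks actor on BeginPlay while a saved guitar-dialog flag is false.
; Box overlap reads three save slots to choose the intro dialogue, an E-key prompt or a roof widget.
; The intro and E-triggered dialogues lock input, poll character flags through 0.2-second Delay loops, then restore input and save progress.
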(event OnComponentBeginOverlap(Box)
  (params (OverlappedComponent :type Primitive%20Component%20Object%20Reference) (OtherActor :type Actor%20Object%20Reference) (OtherComp :type Primitive%20Component%20Object%20Reference) (OtherBodyIndex :type Integer) (bFromSweep :type Boolean) (SweepResult :type Hit%20Result%20Structure%20%28by%20ref%29))
  (Utilities|Casting|CastToBP_Character OtherActor)
  (Utilities|FlowControl|Sequence
    (:then_0
      (bind _returnvalue (SaveGame|LoadGamefromSlot "poimka"))
      (bind _asbp_save_main_character (Utilities|Casting|CastToBP_saveMainCharacter _returnvalue))
      (Utilities|FlowControl|Delay 0.2)
      (if (Variables|/Game/Blueprint/Main_Character/BP_saveMainCharacter.BP_saveMainCharacter_C|GetdialogPeredKrish (stale _asbp_save_main_character_3))
        (if (not (Variables|/Game/Blueprint/Main_Character/BP_saveMainCharacter.BP_saveMainCharacter_C|Getgitardialog (stale _asbp_save_main_character_2)))
          (if (Variables|/Game/Blueprint/Main_Character/BP_saveMainCharacter.BP_saveMainCharacter_C|GetnePaimal _asbp_save_main_character)
            (bind _returnvalue_2 (UserInterface|CreateWidget "/Game/Blueprint/Teleport/WereTicket/WBP_dialogWereTicket.WBP_dialogWereTicket_C"))
            (UserInterface|Viewport|AddtoViewport _returnvalue_2 0)
            (Input|EnableInput (Game|GetPlayerController 0))
            (else
              (bind _returnvalue_3 (UserInterface|CreateWidget "/Game/Blueprint/Teleport/music/quest/WBP_naKrishe.WBP_naKrishe_C"))
              (UserInterface|Viewport|AddtoViewport _returnvalue_3 0))))
        (else
          (bind _asbp_character (Utilities|Casting|CastToBP_Character (Game|GetPlayerCharacter 0)))
          (Input|DisableInput _asbp_character (Game|GetPlayerController 0))
          (bind _returnvalue_4 (UserInterface|CreateWidget "/Game/Blueprint/Teleport/music/quest/WBP_start_music.WBP_start_music_C"))
          (UserInterface|Viewport|AddtoViewport _returnvalue_4 0)
          (if (Variables|/Game/Blueprint/Main_Character/BP_Character.BP_Character_C|GetdialogPeredKrish _asbp_character) :!label _label
            (Input|EnableInput _asbp_character 0)
            (bind _returnvalue_5 (SaveGame|CreateSaveGameObject "/Game/Blueprint/Main_Character/BP_saveMainCharacter.BP_saveMainCharacter_C"))
            (Variables|/Game/Blueprint/Main_Character/BP_saveMainCharacter.BP_saveMainCharacter_C|SetdialogPeredKrish _returnvalue_5 (Variables|/Game/Blueprint/Main_Character/BP_Character.BP_Character_C|GetdialogPeredKrish _asbp_character))
            (SaveGame|SaveGametoSlot _returnvalue_5 "peredkrisha")
            (Audio|PlaySound2D "/Game/Blueprint/Teleport/widget_subtitri/Speakers/Gta5_sound.Gta5_sound" 1.0 1.0 0.0 0 0)
            (bind _returnvalue_6 (UserInterface|CreateWidget "/Game/Blueprint/Teleport/music/quest/WBP_music_sposob.WBP_music_sposob_C"))
            (UserInterface|Viewport|AddtoViewport _returnvalue_6 0)
            (Utilities|FlowControl|Delay 2.0)
            (Widget|RemovefromParent _returnvalue_6)
            (else
              (Utilities|FlowControl|Delay 0.2)
              (goto _label))))))
    (:then_1
      (bind _returnvalue_7 (SaveGame|LoadGamefromSlot "gitarDialog"))
      (bind _asbp_save_main_character_2 (Utilities|Casting|CastToBP_saveMainCharacter _returnvalue_7)))
    (:then_2
      (bind _returnvalue_8 (SaveGame|LoadGamefromSlot "peredkrisha"))
      (bind _asbp_save_main_character_3 (Utilities|Casting|CastToBP_saveMainCharacter _returnvalue_8)))))

(event OnComponentEndOverlap(Box)
  (params (OverlappedComponent :type Primitive%20Component%20Object%20Reference) (OtherActor :type Actor%20Object%20Reference) (OtherComp :type Primitive%20Component%20Object%20Reference) (OtherBodyIndex :type Integer))
  (Utilities|Casting|CastToBP_Character OtherActor)
  (Widget|RemovefromParent (stale OnComponentBeginOverlap(Box) _returnvalue_2))
  (Input|DisableInput (Game|GetPlayerController 0)))

(event EventBeginPlay
  (Utilities|Casting|CastToBP_Character (Game|GetPlayerCharacter 0))
  (Utilities|FlowControl|Sequence
    (:then_0
      (bind _returnvalue (SaveGame|DoesSaveGameExist "gitarDialog"))
      (if _returnvalue
        (bind _returnvalue_2 (SaveGame|LoadGamefromSlot "gitarDialog"))
        (bind _asbp_save_main_character (Utilities|Casting|CastToBP_saveMainCharacter _returnvalue_2))
        (if (not (Variables|/Game/Blueprint/Main_Character/BP_saveMainCharacter.BP_saveMainCharacter_C|Getgitardialog _asbp_save_main_character))
          (Game|SpawnActorfromClass "/Game/Blueprint/Markers/BP_marks.BP_marks_C" (Math|Conversions|ToTransform(Vector) (Transformation|GetWorldLocation (Variables|Default|GetBox))) "Undefined" "MultiplyWithRoot" 0 0))))
    (:then_1
      (bind _returnvalue_3 (SaveGame|DoesSaveGameExist "poimka"))
      (if _returnvalue_3
        (bind _returnvalue_4 (SaveGame|LoadGamefromSlot "poimka"))
        (bind _asbp_save_main_character_2 (Utilities|Casting|CastToBP_saveMainCharacter _returnvalue_4))))
    (:then_2
      (bind _returnvalue_5 (SaveGame|DoesSaveGameExist "peredkrisha"))
      (if _returnvalue_5
        (bind _returnvalue_6 (SaveGame|LoadGamefromSlot "peredkrisha"))
        (bind _asbp_save_main_character_3 (Utilities|Casting|CastToBP_saveMainCharacter _returnvalue_6))))))

(event Input|KeyboardEvents|E
  (params (Key :type Key%20Structure :default "None"))
  (:Pressed
    (if (not (Variables|Default|Getb))
      (Variables|Default|Setb true)
      (Widget|RemovefromParent (stale OnComponentBeginOverlap(Box) _returnvalue_2))
      (bind _asbp_character (Utilities|Casting|CastToBP_Character (Game|GetPlayerCharacter 0)))
      (Input|DisableInput _asbp_character (Game|GetPlayerController 0))
      (bind _returnvalue (UserInterface|CreateWidget "/Game/Blueprint/Teleport/music/quest/poimal/WBP_poimal.WBP_poimal_C"))
      (UserInterface|Viewport|AddtoViewport _returnvalue 0)
      (if (Variables|/Game/Blueprint/Main_Character/BP_Character.BP_Character_C|GetgitarDialog _asbp_character) :!label _label
        (Input|EnableInput _asbp_character 0)
        (bind _returnvalue_2 (SaveGame|CreateSaveGameObject "/Game/Blueprint/Main_Character/BP_saveMainCharacter.BP_saveMainCharacter_C"))
        (Variables|/Game/Blueprint/Main_Character/BP_saveMainCharacter.BP_saveMainCharacter_C|Setgitardialog _returnvalue_2 (Variables|/Game/Blueprint/Main_Character/BP_Character.BP_Character_C|GetgitarDialog _asbp_character))
        (SaveGame|SaveGametoSlot _returnvalue_2 "gitarDialog")
        (else
          (Utilities|FlowControl|Delay 0.2)
          (goto _label))))))

(fn ConstructionScript)