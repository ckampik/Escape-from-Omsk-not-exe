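; PaperZD animation notify that lands the main character's light attack hit during a 2D animation sequence.
; On notify, it box-overlaps Pawns at the sequence render component's location, ignores the owning actor, and applies fixed damage to each hit.
; Without a valid owning instance, as in editor preview, it only draws a debug box of the same extent.
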(event EventOnReceiveNotify
  (params (OwningInstance :type Paper%20ZD%20Anim%20Instance%20Object%20Reference))
  (Utilities|IsValid OwningInstance
    (:Is%20Valid
      (bind _outactors (Collision|BoxOverlapActors (Transformation|GetWorldLocation (Variables|Default|GetSequenceRenderComponent)) (Variables|Default|GetExtent) (Utilities|Array|MakeArray "ObjectTypeQuery3") 0 (Utilities|Array|MakeArray (Class|PaperZDAnimInstance|GetOwningActor OwningInstance)) :!class /Script/Engine.KismetSystemLibrary))
      (for _array_element _outactors
        (Game|Damage|ApplyDamage _array_element 4e+01 0 0)))
    (:Is%20Not%20Valid
      (Rendering|Debug|DrawDebugBox :Center (Transformation|GetWorldLocation (Variables|Default|GetSequenceRenderComponent)) :Extent (Variables|Default|GetExtent)))))

(fn NewFunction)