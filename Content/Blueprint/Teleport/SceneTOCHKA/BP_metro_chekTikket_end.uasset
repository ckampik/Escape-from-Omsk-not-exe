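; Metro trigger actor that checks for a ticket at the end of the TOCHKA scene.
; When BP_Character enters the box, it loads the SaveScene1 and HaveTicket save slots, using a short delay so both are read before checking.
; With Scene1 set and a ticket held, it disables input, plays a sound and fades into the last-metro widget.
; Without a ticket, it shows a scene-end widget, removed on leaving the box.
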(event OnComponentBeginOverlap(Box)
  (params (OverlappedComponent :type Primitive%20Component%20Object%20Reference) (OtherActor :type Actor%20Object%20Reference) (OtherComp :type Primitive%20Component%20Object%20Reference) (OtherBodyIndex :type Integer) (bFromSweep :type Boolean) (SweepResult :type Hit%20Result%20Structure%20%28by%20ref%29))
  (Utilities|Casting|CastToBP_Character OtherActor)
  (Utilities|FlowControl|Sequence
    (:then_0
      (bind _returnvalue (SaveGame|LoadGamefromSlot "SaveScene1"))
      (bind _asbp_save_main_character (Utilities|Casting|CastToBP_saveMainCharacter _returnvalue))
      (Utilities|FlowControl|Delay 0.2)
      (if (Variables|/Game/Blueprint/Main_Character/BP_saveMainCharacter.BP_saveMainCharacter_C|Getscene1 _asbp_save_main_character)
        (if (Variables|/Game/Blueprint/Main_Character/BP_saveMainCharacter.BP_saveMainCharacter_C|GetiHaveTicket (stale _asbp_save_main_character_2))
          (bind _asbp_character (Utilities|Casting|CastToBP_Character (Game|GetPlayerCharacter 0)))
          (Input|DisableInput _asbp_character (Game|GetPlayerController 0))
          (Utilities|FlowControl|Sequence
            (:then_0
              (bind _returnvalue_2 (UserInterface|CreateWidget "/Game/Blueprint/Teleport/WBP_fade.WBP_fade_C"))
              (UserInterface|Viewport|AddtoViewport _returnvalue_2 0)
              (Utilities|FlowControl|Sequence
                (:then_0
                  (Utilities|FlowControl|Delay 2.0)
                  (bind _returnvalue_3 (UserInterface|CreateWidget "/Game/Maps/CinematicKatScene/WBP_lastMetro.WBP_lastMetro_C"))
                  (UserInterface|Viewport|AddtoViewport _returnvalue_3 0))
                (:then_1
                  (Utilities|FlowControl|Delay 2.0)
                  (Widget|RemovefromParent _returnvalue_2))))
            (:then_1
              (Audio|PlaySound2D "/Game/Maps/CinematicKatScene/edu.edu" 1.0 1.0 0.0 0 0)))
          (else
            (bind _returnvalue_4 (UserInterface|CreateWidget "/Game/Blueprint/Teleport/SceneTOCHKA/WBP_TOCHKA_scene_end.WBP_TOCHKA_scene_end_C"))
            (UserInterface|Viewport|AddtoViewport _returnvalue_4 0)))))
    (:then_1
      (bind _returnvalue_5 (SaveGame|LoadGamefromSlot "HaveTicket"))
      (bind _asbp_save_main_character_2 (Utilities|Casting|CastToBP_saveMainCharacter _returnvalue_5)))))

(event OnComponentEndOverlap(Box)
  (params (OverlappedComponent :type Primitive%20Component%20Object%20Reference) (OtherActor :type Actor%20Object%20Reference) (OtherComp :type Primitive%20Component%20Object%20Reference) (OtherBodyIndex :type Integer))
  (Utilities|Casting|CastToBP_Character OtherActor)
  (Widget|RemovefromParent (stale OnComponentBeginOverlap(Box) _returnvalue_4)))

(event EventBeginPlay
  (Utilities|FlowControl|Sequence
    (:then_0
      (bind _returnvalue (SaveGame|DoesSaveGameExist "SaveScene1"))
      (if _returnvalue
        (bind _returnvalue_2 (SaveGame|LoadGamefromSlot "SaveScene1"))
        (bind _asbp_save_main_character (Utilities|Casting|CastToBP_saveMainCharacter _returnvalue_2))))
    (:then_1
      (bind _returnvalue_3 (SaveGame|DoesSaveGameExist "HaveTicket"))
      (if _returnvalue_3
        (bind _returnvalue_4 (SaveGame|LoadGamefromSlot "HaveTicket"))
        (bind _asbp_save_main_character_2 (Utilities|Casting|CastToBP_saveMainCharacter _returnvalue_4))))))

(fn ConstructionScript)