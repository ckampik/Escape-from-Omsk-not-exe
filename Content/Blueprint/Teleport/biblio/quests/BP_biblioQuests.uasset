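; Library quest trigger that lets the player collect notes, tracked through save slots.
; On BeginPlay it spawns a marker and notes actor if the HaveNotes save exists with its flag false.
; Box overlap checks both saves after a short delay and, once the guitar dialog flag is set, plays a sound and shows one of two quest widgets.
; Pressing E saves the notes flag and destroys the notes.
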(event OnComponentEndOverlap(Box)
  (params (OverlappedComponent :type Primitive%20Component%20Object%20Reference) (OtherActor :type Actor%20Object%20Reference) (OtherComp :type Primitive%20Component%20Object%20Reference) (OtherBodyIndex :type Integer))
  (Utilities|Casting|CastToBP_Character OtherActor)
  (Widget|RemovefromParent (stale OnComponentBeginOverlap(Box) _returnvalue_2))
  (Input|DisableInput (Game|GetPlayerController 0)))

(event OnComponentBeginOverlap(Box)
  (params (OverlappedComponent :type Primitive%20Component%20Object%20Reference) (OtherActor :type Actor%20Object%20Reference) (OtherComp :type Primitive%20Component%20Object%20Reference) (OtherBodyIndex :type Integer) (bFromSweep :type Boolean) (SweepResult :type Hit%20Result%20Structure%20%28by%20ref%29))
  (Utilities|Casting|CastToBP_Character OtherActor)
  ;[0 0 0] BRANCH SAVE
  (Utilities|FlowControl|Sequence
    (:then_0
      (bind _returnvalue (SaveGame|LoadGamefromSlot "HaveNotes"))
      (bind _asbp_save_main_character (Utilities|Casting|CastToBP_saveMainCharacter _returnvalue))
      (Utilities|FlowControl|Delay 0.2)
      (if (Variables|/Game/Blueprint/Main_Character/BP_saveMainCharacter.BP_saveMainCharacter_C|Getgitardialog (stale _asbp_save_main_character_2))
        (if (Variables|/Game/Blueprint/Main_Character/BP_saveMainCharacter.BP_saveMainCharacter_C|GetiHaveNotes _asbp_save_main_character)
          (Audio|PlaySound2D "/Game/Blueprint/Teleport/widget_subtitri/Speakers/Gta5_sound.Gta5_sound" 1.0 1.0 0.0 0 0)
          (bind _returnvalue_2 (UserInterface|CreateWidget "/Game/Blueprint/Teleport/biblio/quests/WBP_biblio_quest1.WBP_biblio_quest1_C"))
          (UserInterface|Viewport|AddtoViewport _returnvalue_2 0)
          (else
            (Audio|PlaySound2D "/Game/Blueprint/Teleport/widget_subtitri/Speakers/Gta5_sound.Gta5_sound" 1.0 1.0 0.0 0 0)
            (bind _returnvalue_3 (UserInterface|CreateWidget "/Game/Blueprint/Teleport/biblio/quests/WBP_biblio_quest.WBP_biblio_quest_C"))
            (UserInterface|Viewport|AddtoViewport _returnvalue_3 0)
            (Input|EnableInput (Game|GetPlayerController 0))))))
    (:then_1
      (bind _returnvalue_4 (SaveGame|LoadGamefromSlot "gitarDialog"))
      (bind _asbp_save_main_character_2 (Utilities|Casting|CastToBP_saveMainCharacter _returnvalue_4)))))

(event EventBeginPlay
  (Utilities|Casting|CastToBP_Character (Game|GetPlayerCharacter 0))
  (Utilities|FlowControl|Sequence
    (:then_0
      ;[0 0 0] BRANCH SAVE
      (bind _returnvalue (SaveGame|DoesSaveGameExist "HaveNotes"))
      (if _returnvalue
        (bind _returnvalue_2 (SaveGame|LoadGamefromSlot "HaveNotes"))
        (bind _asbp_save_main_character (Utilities|Casting|CastToBP_saveMainCharacter _returnvalue_2))
        (if (not (Variables|/Game/Blueprint/Main_Character/BP_saveMainCharacter.BP_saveMainCharacter_C|GetiHaveNotes _asbp_save_main_character))
          (Game|SpawnActorfromClass "/Game/Blueprint/Markers/BP_marks.BP_marks_C" (Math|Conversions|ToTransform(Vector) (Transformation|GetWorldLocation (Variables|Default|GetBox))) "Undefined" "MultiplyWithRoot" 0 0)
          (bind _returnvalue_3 (Game|SpawnActorfromClass "/Game/Blueprint/Teleport/biblio/quests/BP_nots.BP_nots_C" (Math|Transform|MakeTransform "5760.000000,-10.000000,510.000000" "0, 0, 0" "1.000000,1.000000,1.000000") "Undefined" "MultiplyWithRoot" 0 0))
          (Variables|Default|Setnotes _returnvalue_3))))
    (:then_1
      (bind _returnvalue_4 (SaveGame|DoesSaveGameExist "gitarDialog"))
      (if _returnvalue_4
        (bind _returnvalue_5 (SaveGame|LoadGamefromSlot "gitarDialog"))
        (bind _asbp_save_main_character_2 (Utilities|Casting|CastToBP_saveMainCharacter _returnvalue_5))))))

(event Input|KeyboardEvents|E
  (params (Key :type Key%20Structure :default "None"))
  (:Pressed
    (Widget|RemovefromParent (stale OnComponentBeginOverlap(Box) _returnvalue_3))
    (bind _returnvalue (SaveGame|CreateSaveGameObject "/Game/Blueprint/Main_Character/BP_saveMainCharacter.BP_saveMainCharacter_C"))
    (Variables|/Game/Blueprint/Main_Character/BP_saveMainCharacter.BP_saveMainCharacter_C|SetiHaveNotes _returnvalue true)
    (SaveGame|SaveGametoSlot _returnvalue "HaveNotes")
    (Actor|DestroyActor (Variables|Default|Getnotes))))

(fn ConstructionScript)