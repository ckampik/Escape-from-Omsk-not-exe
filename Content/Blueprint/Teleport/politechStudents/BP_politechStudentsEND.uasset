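; BP_politechStudentsEND is a trigger box that shows an ending widget for the politech students scene.
; On player overlap it loads the SaveScene3 and HaveGitar saves, using a short delay so both load before checking.
; If SceneStudents is set, IHaveGitar picks the widget, and having the guitar also spawns a teleport to poli street out.
; End overlap removes the widgets; the BeginPlay save loads go unused.
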(event OnComponentEndOverlap(Box)
  (params (OverlappedComponent :type Primitive%20Component%20Object%20Reference) (OtherActor :type Actor%20Object%20Reference) (OtherComp :type Primitive%20Component%20Object%20Reference) (OtherBodyIndex :type Integer))
  (Utilities|Casting|CastToBP_Character OtherActor)
  (Widget|RemovefromParent (stale OnComponentBeginOverlap(Box) _returnvalue_3)))

(event OnComponentBeginOverlap(Box)
  (params (OverlappedComponent :type Primitive%20Component%20Object%20Reference) (OtherActor :type Actor%20Object%20Reference) (OtherComp :type Primitive%20Component%20Object%20Reference) (OtherBodyIndex :type Integer) (bFromSweep :type Boolean) (SweepResult :type Hit%20Result%20Structure%20%28by%20ref%29))
  (Utilities|Casting|CastToBP_Character OtherActor)
  (Utilities|FlowControl|Sequence
    (:then_0
      ;[0 0 0] BRANCH SAVE
      (bind _returnvalue (SaveGame|LoadGamefromSlot "SaveScene3"))
      (bind _asbp_save_main_character (Utilities|Casting|CastToBP_saveMainCharacter _returnvalue))
      (Utilities|FlowControl|Delay 0.2)
      (if (Variables|/Game/Blueprint/Main_Character/BP_saveMainCharacter.BP_saveMainCharacter_C|GetsceneStudents _asbp_save_main_character)
        (if (Variables|/Game/Blueprint/Main_Character/BP_saveMainCharacter.BP_saveMainCharacter_C|GetiHaveGitar (stale _asbp_save_main_character_2))
          (bind _returnvalue_2 (UserInterface|CreateWidget "/Game/Blueprint/Teleport/politechStudents/WBP_studentEND_HaveGitar.WBP_studentEND_HaveGitar_C"))
          (UserInterface|Viewport|AddtoViewport _returnvalue_2 0)
          (Game|SpawnActorfromClass "/Game/Blueprint/Teleport/politech/BP_teleport_to_poli_street_out.BP_teleport_to_poli_street_out_C" (Math|Transform|MakeTransform "1790.929063,-2.700006,-727.976164" "0, 0, 0" "6.554526,1.000000,1.000000") "Undefined" "MultiplyWithRoot" 0 0)
          (else
            (bind _returnvalue_3 (UserInterface|CreateWidget "/Game/Blueprint/Teleport/politechStudents/WBP_studentENDEND.WBP_studentENDEND_C"))
            (UserInterface|Viewport|AddtoViewport _returnvalue_3 0)))))
    (:then_1
      (bind _returnvalue_4 (SaveGame|LoadGamefromSlot "HaveGitar"))
      (bind _asbp_save_main_character_2 (Utilities|Casting|CastToBP_saveMainCharacter _returnvalue_4)))))

(event EventBeginPlay
  (Utilities|FlowControl|Sequence
    (:then_0
      (bind _returnvalue (SaveGame|DoesSaveGameExist "SaveScene3"))
      (if _returnvalue
        (bind _returnvalue_2 (SaveGame|LoadGamefromSlot "SaveScene3"))
        (bind _asbp_save_main_character (Utilities|Casting|CastToBP_saveMainCharacter _returnvalue_2))))
    (:then_1
      (bind _returnvalue_3 (SaveGame|DoesSaveGameExist "HaveGitar"))
      (if _returnvalue_3
        (bind _returnvalue_4 (SaveGame|LoadGamefromSlot "HaveGitar"))
        (bind _asbp_save_main_character_2 (Utilities|Casting|CastToBP_saveMainCharacter _returnvalue_4))))))

(fn ConstructionScript)