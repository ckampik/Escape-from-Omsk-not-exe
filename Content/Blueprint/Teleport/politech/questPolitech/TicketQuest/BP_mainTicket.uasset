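; BP_mainTicket is the interaction point for a ticket quest, using the HaveTicket save slot to track whether the player has the ticket.
; When a save exists without the ticket, it spawns a BP_marks at BeginPlay and shows a dialog prompt with sound on box overlap; with the ticket, overlap shows an end widget.
; Pressing E once opens the quest widget, freezes the character, polls IHaveTicket via a Delay loop, then restores input and saves.
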(event OnComponentBeginOverlap(Box)
  (params (OverlappedComponent :type Primitive%20Component%20Object%20Reference) (OtherActor :type Actor%20Object%20Reference) (OtherComp :type Primitive%20Component%20Object%20Reference) (OtherBodyIndex :type Integer) (bFromSweep :type Boolean) (SweepResult :type Hit%20Result%20Structure%20%28by%20ref%29))
  (Utilities|Casting|CastToBP_Character OtherActor)
  (bind _returnvalue (SaveGame|DoesSaveGameExist "HaveTicket"))
  (if _returnvalue
    (bind _returnvalue_2 (SaveGame|LoadGamefromSlot "HaveTicket"))
    (bind _asbp_save_main_character (Utilities|Casting|CastToBP_saveMainCharacter _returnvalue_2))
    (if (Variables|/Game/Blueprint/Main_Character/BP_saveMainCharacter.BP_saveMainCharacter_C|GetiHaveTicket _asbp_save_main_character)
      (bind _returnvalue_3 (UserInterface|CreateWidget "/Game/Blueprint/Teleport/politech/questPolitech/TicketQuest/WBP_mainTicketEND.WBP_mainTicketEND_C"))
      (UserInterface|Viewport|AddtoViewport _returnvalue_3 0)
      (else
        (Audio|PlaySound2D "/Game/Blueprint/Teleport/widget_subtitri/Speakers/Gta5_sound.Gta5_sound" 1.0 1.0 0.0 0 0)
        (bind _returnvalue_4 (UserInterface|CreateWidget "/Game/Blueprint/Teleport/politech/questPolitech/TicketQuest/WBP_start_dialog.WBP_start_dialog_C"))
        (UserInterface|Viewport|AddtoViewport _returnvalue_4 0)
        (Input|EnableInput (Game|GetPlayerController 0))))))

(event OnComponentEndOverlap(Box)
  (params (OverlappedComponent :type Primitive%20Component%20Object%20Reference) (OtherActor :type Actor%20Object%20Reference) (OtherComp :type Primitive%20Component%20Object%20Reference) (OtherBodyIndex :type Integer))
  (Utilities|Casting|CastToBP_Character OtherActor)
  (Widget|RemovefromParent (stale OnComponentBeginOverlap(Box) _returnvalue_4))
  (Input|DisableInput (Game|GetPlayerController 0)))

(event EventBeginPlay
  (Utilities|Casting|CastToBP_Character (Game|GetPlayerCharacter 0))
  (bind _returnvalue (SaveGame|DoesSaveGameExist "HaveTicket"))
  (if _returnvalue
    (bind _returnvalue_2 (SaveGame|LoadGamefromSlot "HaveTicket"))
    (bind _asbp_save_main_character (Utilities|Casting|CastToBP_saveMainCharacter _returnvalue_2))
    (if (not (Variables|/Game/Blueprint/Main_Character/BP_saveMainCharacter.BP_saveMainCharacter_C|GetiHaveTicket _asbp_save_main_character))
      (Game|SpawnActorfromClass "/Game/Blueprint/Markers/BP_marks.BP_marks_C" (Math|Conversions|ToTransform(Vector) (Transformation|GetWorldLocation (Variables|Default|GetBox))) "Undefined" "MultiplyWithRoot" 0 0))))

(event Input|KeyboardEvents|E
  (params (Key :type Key%20Structure :default "None"))
  (bind _returnvalue (Game|GetPlayerController 0))
  (:Pressed
    (if (not (Variables|Default|Getb))
      (Variables|Default|Setb true)
      (Widget|RemovefromParent (stale OnComponentBeginOverlap(Box) _returnvalue_4))
      (bind _asbp_character (Utilities|Casting|CastToBP_Character (Game|GetPlayerCharacter 0)))
      (Input|DisableInput _asbp_character _returnvalue)
      (bind _returnvalue_2 (UserInterface|CreateWidget "/Game/Blueprint/Teleport/politech/questPolitech/TicketQuest/WBP_mainTicket.WBP_mainTicket_C"))
      (UserInterface|Viewport|AddtoViewport _returnvalue_2 0)
      (if (Variables|/Game/Blueprint/Main_Character/BP_Character.BP_Character_C|GetiHaveTicket _asbp_character) :!label _label
        (Input|EnableInput _asbp_character _returnvalue)
        (bind _returnvalue_3 (SaveGame|CreateSaveGameObject "/Game/Blueprint/Main_Character/BP_saveMainCharacter.BP_saveMainCharacter_C"))
        (Variables|/Game/Blueprint/Main_Character/BP_saveMainCharacter.BP_saveMainCharacter_C|SetiHaveTicket _returnvalue_3 (Variables|/Game/Blueprint/Main_Character/BP_Character.BP_Character_C|GetiHaveTicket _asbp_character))
        (SaveGame|SaveGametoSlot _returnvalue_3 "HaveTicket")
        (else
          (Utilities|FlowControl|Delay 0.2)
          (goto _label))))))

(fn ConstructionScript)